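; Test PVP game mode that starts a two-player match on WildGameState once enough players have joined.
; After each login it waits briefly, then calls StartGame if at least two players are present, with no guard against repeat starts.
; StartGame passes the first two PlayerControllers found in the world to InitPlayers as P1 and P2, then calls StartGame on the game state.
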(event Custom|StartGame
  (bind _aswild_game_state (Utilities|Casting|CastToWildGameState (Game|GetGameState)))
  (bind _outactors (Actor|GetAllActorsOfClass "/Script/Engine.PlayerController"))
  (Class|WildGameState|InitPlayers _aswild_game_state (Utilities|Array|Get(acopy) _outactors) (Utilities|Array|Get(acopy) _outactors 1))
  (Class|WildGameState|StartGame _aswild_game_state))

(event EventBeginPlay)

(event EventTick
  (params (DeltaSeconds :type Float%20%28single-precision%29)))

(event EventPostLogin
  (params (NewPlayer :type Player%20Controller%20Object%20Reference))
  (Utilities|FlowControl|Delay 0.1)
  (bind _returnvalue (Class|GameModeBase|GetNumPlayers))
  (if (>= _returnvalue 2)
    (CallFunction|StartGame)))

(fn ConstructionScript)