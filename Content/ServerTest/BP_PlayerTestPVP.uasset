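; BP_PlayerTestPVP is a test player actor that moves by mouse edge scrolling.
; Each Tick it checks whether the cursor is in the outer tenth of the viewport on any side.
; If so, it offsets the actor in world X and Z by the cursor's offset from screen center times delta time, with screen Y inverted, so speed grows with distance from center.
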(event EventBeginPlay)

(event Collision|EventActorBeginOverlap
  (params (OtherActor :type Actor%20Object%20Reference)))

(event EventTick
  (params (DeltaSeconds :type Float%20%28single-precision%29))
  (bind _returnvalue (Game|GetPlayerController 0))
  (bind _returnvalue_2 (Viewport|GetViewportSize))
  (bind (_locationx _locationy) (Game|Player|GetMousePosition _returnvalue))
  (bind _returnvalue_3 (/ _locationx (.x _returnvalue_2)))
  (bind _returnvalue_4 (/ _locationy (.y _returnvalue_2)))
  (bind _output_get (Variables|Default|SetCentorPos (Math|Vector2D|MakeVector2D (/ (.x _returnvalue_2) 2.0) (/ (.y _returnvalue_2) 2.0))))
  (if (Math|Boolean|ORBoolean (> _returnvalue_3 0.9) (< _returnvalue_3 0.1) (> _returnvalue_4 0.9) (< _returnvalue_4 0.1))
    (Class|Actor|AddActorWorldTransform (Math|Transform|MakeTransform (Math|Vector|MakeVector (.x (* (- (Math|Vector2D|MakeVector2D _locationx _locationy) _output_get) DeltaSeconds)) 0.0 (* (.y (* (- (Math|Vector2D|MakeVector2D _locationx _locationy) _output_get) DeltaSeconds)) -1.0)) "0, 0, 0" "1.000000,1.000000,1.000000") false false)))

(fn ConstructionScript)