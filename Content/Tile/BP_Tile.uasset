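; BP_Tile is a tile actor with a cube mesh that reacts to the mouse cursor.
; Hovering switches player 0's cursor to a hand and turns the cube blue, and leaving restores the default cursor and basic shape material.
; Clicking only prints a debug message, and the leftover manual event-binding nodes never run.
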(event OnBeginCursorOver(Cube)
  (params (TouchedComponent :type Primitive%20Component%20Object%20Reference))
  (Variables|/Script/Engine.PlayerController|SetCurrentMouseCursor (Game|GetPlayerController 0) "Hand")
  (Rendering|Material|SetMaterial (Variables|Default|GetCube) 0 "/Game/Tile/M_Blue.M_Blue"))

(event OnEndCursorOver(Cube)
  (params (TouchedComponent :type Primitive%20Component%20Object%20Reference))
  (Variables|/Script/Engine.PlayerController|SetCurrentMouseCursor (Game|GetPlayerController 0) "Default")
  (Rendering|Material|SetMaterial (Variables|Default|GetCube) 0 "/Engine/BasicShapes/BasicShapeMaterial.BasicShapeMaterial"))

(event OnClicked(Cube)
  (params (TouchedComponent :type Primitive%20Component%20Object%20Reference) (ButtonPressed :type Key%20Structure :default "None"))
  (Development|PrintText "Clicked"))

(event EventBeginPlay)

(event Collision|EventActorBeginOverlap
  (params (OtherActor :type Actor%20Object%20Reference)))

(event EventTick
  (params (DeltaSeconds :type Float%20%28single-precision%29)))

(fn ConstructionScript)